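; Player controller for a turn-based Host/Guest chat game with winners and limited chances.
; BeginPlay binds the chat window's send event after a delay if a remote role exists.
; Sent messages pass to BP_ChatMode only when HostTurn matches the Host/Guest UserId, otherwise a turn warning prints.
; Authority-only broadcast events print messages, and a win or exhausted FalseCount resets the count and calls the game mode's RandomInt.
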(event `self.ReceiveBeginPlay`
  ; 리슨서버는 서버와 클라 둘 다 하기에 서버일때는 아무것도 안하게 해야함
  ; (안그러면 HOST가 가지고 있는 guest도 같이 보내짐)
  (set `self.HostTurn` true)
  (if (not (`|EnumEquality` (`self.GetRemoteRole`) "ROLE_None"))
    (`KismetSystemLibrary.Delay` 0.5)
    (bind _foundwidgets (`WidgetBlueprintLibrary.GetAllWidgetsOfClass` "/Game/Widgets/Widget_ChatWindow.Widget_ChatWindow_C"))
    (bind _output_get (set `self.Widget` (`|GetArrayItem` _foundwidgets)))
    (bind _aswidget_chat_window (cast `/Game/Widgets/Widget_ChatWindow` _output_get))
    (add `/Game/Widgets/Widget_ChatWindow.SetMessageToUserController` _aswidget_chat_window (`|CreateDelegate` :!event `OnSendMsgToServer`))))

(event `OnLoginWithID`
  (params (UserId :type String))
  (`self.OnUserLogin` UserId)
  (set `self.UserId` UserId))

(event `WindBroadCast`
  (params (Name :type String))
  (if (`self.HasAuthority`)
    (`KismetSystemLibrary.PrintString` (`KismetStringLibrary.Concat_StrStr` Name "가 우승하였습니다. ") true true (struct :`G` 0.66 :`B` 1.0 :`A` 1.0) 10.0)
    (bind _asbp_chat_mode (cast `/Game/GameModes/BP_ChatMode` (`GameplayStatics.GetGameMode`)))
    (`/Game/GameModes/BP_ChatMode.RandomInt` _asbp_chat_mode)
    (set `self.FalseCount` 0)))

(event `GotBroadcast`
  (params (Msg :type String) (Name :type String))
  (if (`self.HasAuthority`)
    (`KismetSystemLibrary.PrintString` Msg true true (struct :`G` 0.66 :`B` 1.0 :`A` 1.0) 10.0)
    (if (== (`self.FalseCount`) 6)
      (`KismetSystemLibrary.PrintString` (`KismetTextLibrary.Conv_TextToString` (`|FormatText` "두 플레이어의 모든 기회가 소진되었습니다. 우승자는 없습니다.")) true true (struct :`G` 0.66 :`B` 1.0 :`A` 1.0) 10.0)
      (set `self.FalseCount` 0)
      (bind _asbp_chat_mode (cast `/Game/GameModes/BP_ChatMode` (`GameplayStatics.GetGameMode`)))
      (`/Game/GameModes/BP_ChatMode.RandomInt` _asbp_chat_mode))))

(event `OnSendMsgToServer`
  (params (Msg :type String))
  (if (`self.HostTurn`)
    (bind _host (`self.ItIsHost`))
    (if _host
      (bind _asbp_chat_mode (cast `/Game/GameModes/BP_ChatMode` (`GameplayStatics.GetGameMode`) :!label _label))
      (`/Game/GameModes/BP_ChatMode.GotMessageFromClient` _asbp_chat_mode Msg (`self.UserId`))
      (else
        (`KismetSystemLibrary.PrintString` "지금은 Host의 차례입니다." true true (struct :`G` 0.66 :`B` 1.0 :`A` 1.0) 3.0)))
    (else
      (bind _host_2 (`self.ItIsHost`))
      (if _host_2
        (`KismetSystemLibrary.PrintString` "지금은 Guest의 차례입니다." true true (struct :`G` 0.66 :`B` 1.0 :`A` 1.0) 3.0)
        (else
          (goto _label))))))

(fn `ItIsHost`
  (returns (Host :type Boolean))
  (if (`KismetStringLibrary.EqualEqual_StrStr` (`self.UserId`) "Host")
    (return true)))

(fn `OnRep_FalseCount`)

(fn `UserConstructionScript`)