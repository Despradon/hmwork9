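; BP_ChatMode is a game mode for a turn-based, chat-driven number baseball game.
; At BeginPlay it stores a random secret, which Verdict compares with each client message.
; It loops over all player controllers, flipping HostTurn, then announces a three-strike win or raises FalseCount and broadcasts the strike/ball/out result.
; TimeOver also flips the turn and prints a Korean timeout notice.
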(event `RandomInt`
  (bind _returnvalue (`MyTestCPPLib.RandomInt`))
  (set `self.Random` _returnvalue))

(event `self.ReceiveBeginPlay`
  (`self.RandomInt`))

(event `GotMessageFromClient`
  (params (Msg :type String) (UserName :type String))
  (bind _output_get (set `self.User Name` UserName))
  (bind _outactors (`GameplayStatics.GetAllActorsOfClass` "/Script/Engine.PlayerController"))
  (for _array_element _outactors
    (bind _asbp_controller (cast `/Game/Blueprints/BP_Controller` _array_element))
    (set `/Game/Blueprints/BP_Controller.HostTurn` (not (`/Game/Blueprints/BP_Controller.HostTurn` _asbp_controller)) _asbp_controller)
    (bind _returnvalue (`MyTestCPPLib.Verdict` (`self.Random`) Msg))
    (if (== (break `BallGameResult` _returnvalue) 3)
      (`/Game/Blueprints/BP_Controller.WindBroadCast` _asbp_controller _output_get)
      (else
        (set `/Game/Blueprints/BP_Controller.FalseCount` (+ (`/Game/Blueprints/BP_Controller.FalseCount` _asbp_controller) 1) _asbp_controller)
        (`/Game/Blueprints/BP_Controller.GotBroadcast` _asbp_controller (`KismetTextLibrary.Conv_TextToString` (`|FormatText` "{strike}S {ball}B {out}O" (break `BallGameResult` _returnvalue) (`.Ball` (break `BallGameResult` _returnvalue)) (`.OutCount` (break `BallGameResult` _returnvalue)))) _output_get)))))

(event `TimeOver`
  (bind _outactors (`GameplayStatics.GetAllActorsOfClass` "/Script/Engine.PlayerController"))
  (for _array_element _outactors
    (bind _asbp_controller (cast `/Game/Blueprints/BP_Controller` _array_element))
    (set `/Game/Blueprints/BP_Controller.HostTurn` (not (`/Game/Blueprints/BP_Controller.HostTurn` _asbp_controller)) _asbp_controller)
    (`KismetSystemLibrary.PrintString` "시간이 초과되었습니다. 상대방에게 기회가 넘어갑니다." true true (struct :`G` 0.66 :`B` 1.0 :`A` 1.0) 5.0)))

(fn `UserConstructionScript`)